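; BP_Enemy is a spinning enemy actor that damages the player on contact and awards score when shot.
; Tick rolls its root steadily, and a sphere overlap handles collisions.
; A BP_Projectile hit increments the owning player's score and destroys both actors.
; A BP_Player hit lowers health, plays a world camera shake, shows restart when health equals zero, and destroys the enemy.
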(event `self.ReceiveTick`
  (params (DeltaSeconds :type "Float (single-precision)"))
  (`SceneComponent.K2_AddLocalRotation` (`self.DefaultSceneRoot`) (`KismetMathLibrary.MakeRotator` (* DeltaSeconds 60.0)) false false))

(event `self.Sphere.OnComponentBeginOverlap`
  (params (OverlappedComponent :type "PrimitiveComponent Object Reference") (OtherActor :type "Actor Object Reference") (OtherComp :type "PrimitiveComponent Object Reference") (OtherBodyIndex :type Integer) (bFromSweep :type Boolean) (SweepResult :type "HitResult Structure (by ref)"))
  (bind _asbp_projectile (cast `/Game/InfiniteMatrix/Blueprints/BP_Projectile` OtherActor)
    (:`then`
      (bind _player (`/Game/InfiniteMatrix/Blueprints/BP_Projectile.Player` _asbp_projectile))
      (set `/Game/InfiniteMatrix/Blueprints/BP_Player.Score` (+ (`/Game/InfiniteMatrix/Blueprints/BP_Player.Score` _player) 1) _player)
      (`/Game/InfiniteMatrix/Blueprints/BP_Player.UpdateScore` _player)
      (`self.K2_DestroyActor`)
      (`self.K2_DestroyActor` _asbp_projectile))
    (:`CastFailed`
      (bind _asbp_player (cast `/Game/InfiniteMatrix/Blueprints/BP_Player` OtherActor))
      (bind _output_get (set `/Game/InfiniteMatrix/Blueprints/BP_Player.Health` (- (`/Game/InfiniteMatrix/Blueprints/BP_Player.Health` _asbp_player) 10) _asbp_player))
      (`/Game/InfiniteMatrix/Blueprints/BP_Player.UpdateHealth` _asbp_player)
      (`GameplayStatics.PlayWorldCameraShake` "/Game/InfiniteMatrix/Blueprints/BP_Shake.BP_Shake_C" (`self.K2_GetActorLocation` _asbp_player) 0.0 500.0)
      (if (== _output_get 0)
        (`/Game/InfiniteMatrix/Blueprints/BP_Player.DisplayRestart` _asbp_player))
      (`self.K2_DestroyActor`))))

(fn `UserConstructionScript`)