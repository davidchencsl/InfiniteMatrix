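; BP_Projectile is a bullet actor that travels in a straight line until it overlaps static geometry.
; Tick offsets it along world X by ForwardSpeed scaled by delta time, independent of the actor's rotation.
; When Bullet begins an overlap, exact class checks skip BP_Player and BP_Enemy, and the projectile destroys itself only if the other component is a StaticMeshComponent.
; It applies no damage itself.
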(event `self.ReceiveBeginPlay`)

(event `self.ReceiveTick`
  (params (DeltaSeconds :type "Float (single-precision)"))
  (`self.K2_AddActorWorldOffset` (`KismetMathLibrary.MakeVector` (* DeltaSeconds (`self.ForwardSpeed`)))))

(event `self.Bullet.OnComponentBeginOverlap`
  (params (OverlappedComponent :type "PrimitiveComponent Object Reference") (OtherActor :type "Actor Object Reference") (OtherComp :type "PrimitiveComponent Object Reference") (OtherBodyIndex :type Integer) (bFromSweep :type Boolean) (SweepResult :type "HitResult Structure (by ref)"))
  (if (!= (`GameplayStatics.GetObjectClass` OtherActor) "/Game/InfiniteMatrix/Blueprints/BP_Player.BP_Player_C")
    (if (!= (`GameplayStatics.GetObjectClass` OtherActor) "/Game/InfiniteMatrix/Blueprints/BP_Enemy.BP_Enemy_C")
      (if (== (`GameplayStatics.GetObjectClass` OtherComp) "/Script/Engine.StaticMeshComponent")
        (`self.K2_DestroyActor`)))))

(fn `UserConstructionScript`)